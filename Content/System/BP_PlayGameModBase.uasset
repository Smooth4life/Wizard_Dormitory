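; BP_PlayGameModBase is the play game mode that handles the end of a day or run by switching levels.
; GameOver opens the game over level directly.
; EndGame opens the clear level when the game instance's CurrentDay equals the DayToNPCCount length.
; Otherwise it copies the NPC total, accepted, fake and rejected counts into BP_GameInstance before opening the stage clear level, so the results persist across the level change.
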(event `self.GameOver`
  (`GameplayStatics.OpenLevelBySoftObjectPtr` "/Game/Maps/M_GameOver.M_GameOver"))

(event `self.EndGame`
  (bind _asbp_game_instance (cast `/Game/System/BP_GameInstance` (`GameplayStatics.GetGameInstance`)))
  (`/Engine/EditorBlueprintResources/StandardMacros.IsValid` _asbp_game_instance
    (:`Is Valid`
      (if (== (`MyGameInstance.CurrentDay` _asbp_game_instance) (`BlueprintMapLibrary.Map_Length` (`MyGameInstance.DayToNPCCount` _asbp_game_instance)))
        (`GameplayStatics.OpenLevelBySoftObjectPtr` "/Game/Maps/M_Clear.M_Clear")
        (else
          (set `/Game/System/BP_GameInstance.Total` (`self.NumNPCToGenerate`) _asbp_game_instance)
          (set `/Game/System/BP_GameInstance.Correct` (`self.NumAccepted`) _asbp_game_instance)
          (set `/Game/System/BP_GameInstance.Fake` (`self.NumFake`) _asbp_game_instance)
          (set `/Game/System/BP_GameInstance.Complain` (`self.NumRejected`) _asbp_game_instance)
          (`GameplayStatics.OpenLevelBySoftObjectPtr` "/Game/Maps/M_StageClear.M_StageClear"))))))

(fn `UserConstructionScript`)