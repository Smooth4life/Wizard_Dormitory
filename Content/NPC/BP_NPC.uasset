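; NPC visitor in a VR ID-checking game that approaches the player, answers questions and gets judged pass or reject.
; It walks waypoint arrays via looping AIMoveTo after a random door, portal or flying entrance.
; Montages, data-table subtitles and hand notifies present the ID card or affiliation effect.
; Yes/No resets the card and props, plays a reaction, walks it out, then reports to the game mode; aiming pulses an overlay outline.
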(event `self.ReceiveBeginPlay`
  (`|ExecutionSequence`
    (:`then_0`
      (bind _asbp_play_game_mod_base (cast `/Game/System/BP_PlayGameModBase` (`GameplayStatics.GetGameMode`)))
      (set `self.As BP Play Game Mod Base` _asbp_play_game_mod_base))
    (:`then_1`
      (bind _asumg_subtitle_root (cast `/Game/Blueprints/UMG/UMG_SubtitleRoot` (`WidgetComponent.GetUserWidgetObject` (`self.Widget`))))
      (set `self.As UMG Subtitle Root` _asumg_subtitle_root))
    (:`then_2`
      (bind _asvrpawn (cast `/Game/Blueprints/VRPawn` (`GameplayStatics.GetPlayerPawn` 0)))
      (set `self.As VRPawn` _asvrpawn))
    (:`then_3`
      (bind _returnvalue (`KismetMaterialLibrary.CreateDynamicMaterialInstance` (`self.M_Highlight_Inst`)))
      (set `self.DMI_Highlight_Inst` _returnvalue))
    (:`then_4`
      (bind _returnvalue_2 (`GameplayStatics.GetActorOfClass` "/Game/Blueprints/BP_IDCard.BP_IDCard_C"))
      (set `self.IDCard` _returnvalue_2))))

(event `self.ReceiveTick`
  (params (DeltaSeconds :type "Float (single-precision)"))
  (if (`self.IsAimed`)
    (`/Engine/EditorBlueprintResources/StandardMacros.DoOnce` false :!label _label
      (:`Completed`
        (`self.Aimed_Highlight`)))
    (else
      (`|ExecutionSequence`
        (:`then_0`
          (goto _label :!via `Reset`))
        (:`then_1`
          (`MeshComponent.SetOverlayMaterial` (`self.Mesh`) null))))))

(event `MoveStart`
  ;[1 1 1] Move To
  (if (`PlayGameModeBase.bGameEnd` (`self.As BP Play Game Mod Base`))
    _
    (elif (`self.bMovemod`)
      (`self.Move` (`self.WaypointStart_2`))
      (else
        (`self.Move` (`self.WaypointStart`))))))

(event `Aimed_Highlight`
  (`MeshComponent.SetOverlayMaterial` (`self.Mesh`) (`self.DMI_Highlight_Inst`))
  (bind (_direction _time) (`Timeline|Timeline_0` :!via `PlayFromStart`)
    (:`Update`
      (`MaterialInstanceDynamic.SetScalarParameterValue` (`self.DMI_Highlight_Inst`) "LineThickness" (`KismetMathLibrary.Lerp` 0.5 3.0 _time)))))

(event `Yes`
  ;[1 1 1] Move To
  (if (not (`self.bIsJudged`))
    (set `self.bIsJudged` true)
    (set `self.bYorN` true)
    ;;[1 1 1] 자막
    (`self.PlayRandomDialogue` "/Game/System/DataTable/DT_Pass.DT_Pass")
    (`self.Anim_Talk`)
    (`self.NPCOut`)
    (`KismetSystemLibrary.Delay` 2.5)
    (if (`self.bLorR`)
      (`self.Move` (`self.WaypointExit_L`))
      (else
        (`self.Move` (`self.WaypointExit_R`))))
    (set `self.bselect` true :!label _label_2)))

(event `No`
  ;[1 1 1] Move To
  (if (not (`self.bIsJudged`))
    (set `self.bIsJudged` true)
    (set `self.bYorN` false)
    ;;[1 1 1] 자막
    (`self.PlayRandomDialogue` "/Game/System/DataTable/DT_Exit.DT_Exit")
    (`self.Anim_Rage`)
    (`self.NPCOut`)
    (`KismetSystemLibrary.Delay` 2.5)
    (`self.Move` (`self.WaypointReturn`))
    (goto _label_2)))

(event `PlayerSelect`
  ;[1 1 1] Select
  (set `self.bselect` false)
  (`|ExecutionSequence`
    (:`then_0`
      (`PlayGameModeBase.EvaluateNPC` (`self.As BP Play Game Mod Base`) (`self.bYorN`)))
    (:`then_1`
      ;;[1 1 1] 플레이어 판단 전달
      ;; 이동이벤트
      (`self.HandleNPCDecision` (`self.bYorN`)))))

(event `Move`
  (params (Array :type "Array of /Game/NPC/BP_TargetPoint Object Reference"))
  (bind _charactermovement (`self.CharacterMovement`))
  (bind _waycount (`self.WayCount`))
  ;[1 1 1] Move
  (set `self.WayCount` 0)
  (`|AIMoveTo` self (0.0 0.0 0.0) (`|GetArrayItem` Array _waycount) :!label _label_3
    (:`OnSuccess`
      (`/Engine/EditorBlueprintResources/StandardMacros.IncrementInt` (`self.WayCount`)
        (:`  `
          (bind _output_get (set `self.bMoveStop` (== (`KismetArrayLibrary.Array_Length` Array) _waycount)))
          (if _output_get
            (if (`self.bselect`)
              (`self.PlayerSelect`)
              (else
                (`/Game/Blueprints/VRPawn.SayHello` (`self.As VRPawn`))))
            (else
              (`|ExecutionSequence`
                (:`then_0`
                  (if (and (!= _waycount 0) (`NavMovementComponent.IsFlying` _charactermovement))
                    (`CharacterMovementComponent.SetMovementMode` _charactermovement "MOVE_Walking" 0)))
                (:`then_1`
                  (goto _label_3))))))))))

(event `show Effect`
  ;[1 1 1] 상징 스폰및 크기 조절
  (`self.ShowAffiliationEffect` (`|GetArrayItem` (`self.AffiliationEffects`) (`self.NPCAffiliationIndex`)))
  (bind (_direction _effectscale) (`Timeline|Timeline` :!via `PlayFromStart`)
    (:`Update`
      (`SceneComponent.SetWorldScale3D` (`self.AffiliationEffectComponent`) (`KismetMathLibrary.Conv_DoubleToVector` _effectscale)))))

(event `self.ShowSubtitle`
  (params (Text :type "Text (by ref)"))
  ;[1 1 1] Subtitle
  (`/Game/Blueprints/UMG/UMG_SubtitleRoot.ShowSubtitle_SubTitleRoot` (`self.As UMG Subtitle Root`) Text false 3.0))

(event `self.StartReturn`
  ;[1 1 1] 랜덤시작위치
  ;;[1 1 1] 입구 도착후 호출
  (set `self.bIsJudged` false)
  (`self.NotifyReturnComplete`)
  (`self.probability` :!label _label_4)
  (switch `int` (`self.Selection`)
    (:`0`
      (`self.DoorStart`))
    (:`1`
      (`self.PortalStart`))
    (:`2`
      (`self.flyStart`))))

(event `On_Notify_HandOn`
  (bind _idcard (`self.IDCard`))
  (if (`self.bIsCard`)
    (`SceneComponent.SetVisibility` (`/Game/Blueprints/BP_IDCard.Card` _idcard) true false)
    (set `/Game/Blueprints/GrabComponent.bIsGrabable` true (`/Game/Blueprints/BP_IDCard.GrabComponentSnapLeft` _idcard))
    (set `/Game/Blueprints/GrabComponent.bIsGrabable` true (`/Game/Blueprints/BP_IDCard.GrabComponentSnapRight` _idcard))
    (`SceneComponent.K2_SetWorldTransform` (`/Game/Blueprints/BP_IDCard.DefaultSceneRoot` _idcard) (`/Game/Blueprints/BP_IDCard.DefaultTransform` _idcard) false false)
    (else
      (`self.show Effect`)
      (set `SkeletalMeshComponent.GlobalAnimRateScale` 0.5 (`self.Mesh`)))))

(event `self.StartExit`
  ;[1 1 1] 랜덤시작위치
  ;;[1 1 1] 출구 도착후 호출
  (set `self.bIsJudged` false)
  (`self.NotifyExitComplete`)
  (goto _label_4))

(event `OnSpeakGreeting`
  ;[1 1 1] 상호작용
  ;;[1 1 1] 인사
  (`AnimInstance.Montage_Play` (`SkeletalMeshComponent.GetAnimInstance` (`self.Mesh`)) "/Game/NPC/Animation/Montage/Anim_Hello_Montage.Anim_Hello_Montage" 1.0 "MontageLength" 0.0 true)
  (`self.PlayRandomDialogue` "/Game/System/DataTable/DT_GreetingDialogue.DT_GreetingDialogue")
  (`KismetSystemLibrary.Delay` 3.0)
  (`/Game/Blueprints/VRPawn.AskForIDCard` (`self.As VRPawn`)))

(event `On_Notify_HandOff`
  (if (`self.bIsCard`)
    (set `self.bIsCard` false)
    (else
      (`self.HideAffiliationEffect`)
      (set `SkeletalMeshComponent.GlobalAnimRateScale` 1.0 (`self.Mesh`)))))

(event `OnSubmitIDCard`
  ;[1 1 1] 상호작용
  ;;[1 1 1] 학생증 제출
  (`AnimInstance.Montage_Play` (`SkeletalMeshComponent.GetAnimInstance` (`self.Mesh`)) "/Game/NPC/Animation/Montage/Anim_Symbol_Checking_Montage.Anim_Symbol_Checking_Montage" 1.0 "MontageLength" 0.0 true)
  (`self.PlayRandomDialogue` "/Game/System/DataTable/DT_Handln.DT_Handln"))

(event `DoorStart`
  ;[1 1 1] 시작위치 이동시 이벤트
  (set `self.bMovemod` true)
  (`self.Set Spawn Location`)
  (`KismetSystemLibrary.Delay` 6.0)
  (`self.MoveStart`))

(event `PortalStart`
  ;[1 1 1] 시작위치 이동시 이벤트
  (set `self.bMovemod` false)
  (`NiagaraFunctionLibrary.SpawnSystemAtLocation` "/Game/VFX/Potal/NS_Potal_V2.NS_Potal_V2" (1420.0 -1646.0 132.0) (struct :`Yaw` -30.0))
  (`KismetSystemLibrary.Delay` 3.0)
  (`self.Set Spawn Location`)
  (`self.MoveStart`))

(event `OnSpeakName`
  ;[1 1 1] 상호작용
  ;;[1 1 1] 이름
  (`self.Anim_Talk`)
  (`self.PlayNameDialogue` "/Game/System/DataTable/DT_NameIdentify.DT_NameIdentify"))

(event `OnAffiliation`
  ;[1 1 1] 상호작용
  ;;[1 1 1] 소속 상징 보여주기
  (`AnimInstance.Montage_Play` (`SkeletalMeshComponent.GetAnimInstance` (`self.Mesh`)) "/Game/NPC/Animation/Montage/Anim_Symbol_Checking_Montage.Anim_Symbol_Checking_Montage" 1.0 "MontageLength" 0.0 true))

(event `flyStart`
  ;[1 1 1] 시작위치 이동시 이벤트
  (set `self.bMovemod` false)
  (`CharacterMovementComponent.SetMovementMode` (`self.CharacterMovement`) "MOVE_Flying" 0)
  (`self.MoveStart`)
  (`self.Set Spawn Location`))

(event `OnStudentID`
  ;[1 1 1] 상호작용
  ;;[1 1 1] 학번
  (`self.Anim_Talk`)
  (`self.PlayStudentIDDialogue`))

(fn `Anim_Rage`
  (`AnimInstance.Montage_Play` (`SkeletalMeshComponent.GetAnimInstance` (`self.Mesh`)) (`KismetArrayLibrary.Array_Random` (`self.Montage_Rage`)) 1.0 "MontageLength" 0.0 true))

(fn `Anim_Talk`
  (`AnimInstance.Montage_Play` (`SkeletalMeshComponent.GetAnimInstance` (`self.Mesh`)) (`KismetArrayLibrary.Array_Random` (`self.Montage_Talk`)) 1.0 "MontageLength" 0.0 true))

(fn `NPCOut`
  (bind _idcard (`self.IDCard`))
  (bind _card (`/Game/Blueprints/BP_IDCard.Card` _idcard))
  (`SceneComponent.SetVisibility` _card false false)
  (set `/Game/Blueprints/GrabComponent.bIsGrabable` false (`/Game/Blueprints/BP_IDCard.GrabComponentSnapLeft` _idcard))
  (set `/Game/Blueprints/GrabComponent.bIsGrabable` false (`/Game/Blueprints/BP_IDCard.GrabComponentSnapRight` _idcard))
  (`PrimitiveComponent.SetSimulatePhysics` _card false)
  (`SceneComponent.K2_DetachFromComponent` _card "KeepWorld" "KeepWorld" "KeepWorld" true)
  (`SceneComponent.K2_AttachToComponent` _card (`/Game/Blueprints/BP_IDCard.DefaultSceneRoot` _idcard) "None" "SnapToTarget" "SnapToTarget" "KeepWorld" true)
  (set `self.bIsCard` true)
  (`PrimitiveComponent.SetSimulatePhysics` _card true)
  (bind _returnvalue (`GameplayStatics.GetActorOfClass` "/Game/Blueprints/HoloGen/BP_HologramGenerator.BP_HologramGenerator_C"))
  (`/Game/Blueprints/HoloGen/BP_HologramGenerator.DespawnHolo` _returnvalue)
  (bind _returnvalue_2 (`GameplayStatics.GetActorOfClass` "/Game/Blueprints/BP_CardReader.BP_CardReader_C"))
  (`/Game/Blueprints/BP_CardReader.Light_Off` _returnvalue_2))

(fn `probability`
  (bind _randomspawn (`self.RandomSpawn`))
  (set `self.RandomSpawn` (`KismetMathLibrary.RandomFloatInRange` 0.0 1.0))
  (if (< _randomspawn 0.3)
    (set `self.Selection` 0)
    (elif (< _randomspawn 0.6)
      (set `self.Selection` 1)
      (elif (<= _randomspawn 1.0)
        (set `self.Selection` 2)))))

(fn `Set Spawn Location`
  (`self.K2_SetActorLocation` (`self.K2_GetActorLocation` (`|GetArrayItem` (`self.WaypointSpawn`) (`self.Selection`)))))

(fn `UserConstructionScript`)