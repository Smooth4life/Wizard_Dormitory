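; BP_Wand1 is a wand Blueprint that tracks which interactable the player aims at.
; AimObject runs a hit actor through nested casts for right gate, ID card, NPC, how-to-play object and left gate.
; A match raises IsAimed on that type's stored reference and sets the AimedObject enum.
; Failed casts clear their flag before trying the next type, falling back to a default enum value, so types after a match keep their flags.
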(fn `AimObject`
  (params (HitActor :type "Actor Object Reference"))
  (bind _bp_how_to_play (`self.BP How To Play`))
  (bind _bp_idcard (`self.BP IDCard`))
  (bind _bp_npc (`self.BP NPC`))
  (bind _bp_gate_right (`self.BP_Gate_Right`))
  (bind _bp_gate_left (`self.BP_Gate_Left`))
  (bind _asbp_gate_right (cast `/Game/Blueprints/BP_Gate_Right` HitActor)
    (:`then`
      (`/Engine/EditorBlueprintResources/StandardMacros.IsValid` _asbp_gate_right
        (:`Is Valid`
          (set `/Game/Blueprints/BP_Gate_Right.IsAimed` true (`self.BP_Gate_Right`))
          (set `self.AimedObject` "NewEnumerator5"))))
    (:`CastFailed`
      (`|ExecutionSequence`
        (:`then_0`
          (`/Engine/EditorBlueprintResources/StandardMacros.IsValid` _bp_gate_right
            (:`Is Valid`
              (set `/Game/Blueprints/BP_Gate_Right.IsAimed` false _bp_gate_right))))
        (:`then_1`
          (bind _asbp_idcard (cast `/Game/Blueprints/BP_IDCard` HitActor)
            (:`then`
              (`/Engine/EditorBlueprintResources/StandardMacros.IsValid` _asbp_idcard
                (:`Is Valid`
                  (set `/Game/Blueprints/BP_IDCard.IsAimed` true (`self.BP IDCard`))
                  (set `self.AimedObject` "NewEnumerator2"))))
            (:`CastFailed`
              (`|ExecutionSequence`
                (:`then_0`
                  (`/Engine/EditorBlueprintResources/StandardMacros.IsValid` _bp_idcard
                    (:`Is Valid`
                      (set `/Game/Blueprints/BP_IDCard.IsAimed` false _bp_idcard))))
                (:`then_1`
                  (bind _asbp_npc (cast `/Game/NPC/BP_NPC` HitActor)
                    (:`then`
                      (`/Engine/EditorBlueprintResources/StandardMacros.IsValid` _asbp_npc
                        (:`Is Valid`
                          (set `/Game/NPC/BP_NPC.IsAimed` true (`self.BP NPC`))
                          (set `self.AimedObject` "NewEnumerator6"))))
                    (:`CastFailed`
                      (`|ExecutionSequence`
                        (:`then_0`
                          (`/Engine/EditorBlueprintResources/StandardMacros.IsValid` _bp_npc
                            (:`Is Valid`
                              (set `/Game/NPC/BP_NPC.IsAimed` false _bp_npc))))
                        (:`then_1`
                          (bind _asbp_how_to_play (cast `/Game/Blueprints/BP_HowToPlay` HitActor)
                            (:`then`
                              (`/Engine/EditorBlueprintResources/StandardMacros.IsValid` _asbp_how_to_play
                                (:`Is Valid`
                                  (set `/Game/Blueprints/BP_HowToPlay.IsAimed` true (`self.BP How To Play`))
                                  (set `self.AimedObject` "NewEnumerator7"))))
                            (:`CastFailed`
                              (`|ExecutionSequence`
                                (:`then_0`
                                  (`/Engine/EditorBlueprintResources/StandardMacros.IsValid` _bp_how_to_play
                                    (:`Is Valid`
                                      (set `/Game/Blueprints/BP_HowToPlay.IsAimed` false _bp_how_to_play))))
                                (:`then_1`
                                  (bind _asbp_gate_left (cast `/Game/Blueprints/BP_Gate_Left` HitActor)
                                    (:`then`
                                      (`/Engine/EditorBlueprintResources/StandardMacros.IsValid` _asbp_gate_left
                                        (:`Is Valid`
                                          (set `/Game/Blueprints/BP_Gate_Left.IsAimed` true (`self.BP_Gate_Left`))
                                          (set `self.AimedObject` "NewEnumerator3"))))
                                    (:`CastFailed`
                                      (`|ExecutionSequence`
                                        (:`then_0`
                                          (`/Engine/EditorBlueprintResources/StandardMacros.IsValid` _bp_gate_left
                                            (:`Is Valid`
                                              (set `/Game/Blueprints/BP_Gate_Left.IsAimed` false _bp_gate_left))))
                                        (:`then_1`
                                          (set `self.AimedObject` "NewEnumerator4"))))))))))))))))))))))

(fn `UserConstructionScript`)