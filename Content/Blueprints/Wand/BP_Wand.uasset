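; Grabbable VR wand that activates the aimed ID card, gate or tutorial, or denies entry to an aimed guest NPC.
; Tick traces from the muzzle with a debug line, and AimObject's cast chain flags the hit target and stores AimedObject.
; Clicks play magic effects, then act on that target after a short delay.
; Grabbing enables per-hand input mapping and target ticking; dropping disables them and snaps the mesh back to root.
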(event `self.ReceiveBeginPlay`
  (`KismetSystemLibrary.Delay` 0.2)
  (bind _returnvalue (`GameplayStatics.GetActorOfClass` "/Game/Blueprints/BP_Gate_Left.BP_Gate_Left_C"))
  (set `self.BP_Gate_Left` _returnvalue)
  (bind _returnvalue_2 (`GameplayStatics.GetActorOfClass` "/Game/Blueprints/BP_Gate_Right.BP_Gate_Right_C"))
  (set `self.BP_Gate_Right` _returnvalue_2)
  (bind _returnvalue_3 (`GameplayStatics.GetActorOfClass` "/Game/Blueprints/BP_IDCard.BP_IDCard_C"))
  (set `self.BP IDCard` _returnvalue_3)
  (set `self.OriginTransform` (`self.GetTransform`))
  (bind _outactors (`GameplayStatics.GetAllActorsOfClassWithTag` "/Game/NPC/BP_NPC.BP_NPC_C" "guest"))
  (set `self.BP NPC` (`|GetArrayItem` _outactors))
  (bind _returnvalue_4 (`GameplayStatics.GetActorOfClass` "/Game/Blueprints/BP_CardReader.BP_CardReader_C"))
  (`KismetArrayLibrary.Array_Add` (`self.Actors to Ignore`) _returnvalue_4)
  (bind _returnvalue_5 (`GameplayStatics.GetActorOfClass` "/Game/Blueprints/HoloGen/BP_HologramGenerator.BP_HologramGenerator_C"))
  (`KismetArrayLibrary.Array_Add` (`self.Actors to Ignore`) _returnvalue_5)
  (bind _returnvalue_6 (`GameplayStatics.GetActorOfClass` "/Game/Blueprints/BP_Phone.BP_Phone_C"))
  (`KismetArrayLibrary.Array_Add` (`self.Actors to Ignore`) _returnvalue_6)
  (bind _returnvalue_7 (`GameplayStatics.GetActorOfClass` "/Game/Blueprints/BP_Radio.BP_Radio_C"))
  (`KismetArrayLibrary.Array_Add` (`self.Actors to Ignore`) _returnvalue_7)
  (bind _asvrpawn (cast `/Game/Blueprints/VRPawn` (`GameplayStatics.GetPlayerPawn` 0)))
  (`/Engine/EditorBlueprintResources/StandardMacros.IsValid` _asvrpawn
    (:`Is Valid`
      (set `self.VRPawn` _asvrpawn))))

(event `EnhancedInput|/Game/System/Input/Wand/Action/IA_Wand_Click_Left`
  (params (ActionValue :type Boolean) (ElapsedSeconds :type "Float (double-precision)") (TriggeredSeconds :type "Float (double-precision)") (InputAction :type "InputAction Object Reference" :default "/Game/System/Input/Wand/Action/IA_Wand_Click_Left.IA_Wand_Click_Left"))
  (:`Started`
    (`ActorComponent.Activate` (`self.NS_magic_shot`) true :!label _label)
    (`ActorComponent.Activate` (`self.NS_magic_Charging`) true)
    (`AudioComponent.Play` (`self.SFX_Magic`) 0.0)
    (`KismetSystemLibrary.Delay` 0.2)
    (switch `/Game/Blueprints/Wand/E_Objects` (`self.AimedObject`)
      (:`NewEnumerator2`
        (set `/Game/Blueprints/BP_IDCard.IsActivated` true (`self.BP IDCard`)))
      (:`NewEnumerator3`
        (set `/Game/Blueprints/BP_Gate_Left.IsActivated` true (`self.BP_Gate_Left`)))
      (:`NewEnumerator5`
        (set `/Game/Blueprints/BP_Gate_Right.IsActivated` true (`self.BP_Gate_Right`)))
      (:`NewEnumerator6`
        (`/Game/Blueprints/VRPawn.DenyEntry` (`self.VRPawn`)))
      (:`NewEnumerator7`
        (set `/Game/Blueprints/BP_HowToPlay.IsActivated` true (`self.BP How To Play`))))))

(event `EnhancedInput|/Game/System/Input/Wand/Action/IA_Wand_Click_Right`
  (params (ActionValue :type Boolean) (ElapsedSeconds :type "Float (double-precision)") (TriggeredSeconds :type "Float (double-precision)") (InputAction :type "InputAction Object Reference" :default "/Game/System/Input/Wand/Action/IA_Wand_Click_Right.IA_Wand_Click_Right"))
  (:`Started`
    (goto _label)))

(event `self.ReceiveTick`
  (params (DeltaSeconds :type "Float (single-precision)"))
  (bind _wandmuzzlelocation (`self.WandMuzzleLocation`))
  (bind _returnvalue (`SceneComponent.K2_GetComponentLocation` _wandmuzzlelocation))
  (bind _outhit (`KismetSystemLibrary.LineTraceSingle` _returnvalue (+ _returnvalue (* (`KismetMathLibrary.GetForwardVector` (`SceneComponent.K2_GetComponentRotation` _wandmuzzlelocation)) 10000.0)) "TraceTypeQuery1" false (`self.Actors to Ignore`) "ForOneFrame"))
  (`self.AimObject` (`.HitActor` (`GameplayStatics.BreakHitResult` _outhit))))

(event `HowToPlaySpawn`
  (bind _returnvalue (`GameplayStatics.GetActorOfClass` "/Game/Blueprints/BP_HowToPlay.BP_HowToPlay_C"))
  (set `self.BP How To Play` _returnvalue))

(event `self.GrabComponentLeft.OnGrabbed`
  ;[1 1 1] InputMapping
  (`self.SetActorTickEnabled` true)
  (`self.EnableInput` (`GameplayStatics.GetPlayerController` 0))
  (`EnhancedInputSubsystemInterface.AddMappingContext` (pcsubsystem `EnhancedInputLocalPlayerSubsystem` (`GameplayStatics.GetPlayerController` 0)) "/Game/System/Input/Wand/IMC_Wand_Left.IMC_Wand_Left" 1 (struct))
  (`self.SetActorTickEnabled` true :!label _label_2)
  (`self.SetActorTickEnabled` (`self.BP IDCard`) true)
  (`self.SetActorTickEnabled` (`self.BP_Gate_Right`) true)
  (`self.SetActorTickEnabled` (`self.BP_Gate_Left`) true)
  (`self.SetActorTickEnabled` (`self.BP NPC`) true)
  (bind _bp_how_to_play (`self.BP How To Play`)
    (:`then`
      (`self.SetActorTickEnabled` _bp_how_to_play true))
    (:`else`)))

(event `self.GrabComponentRight.OnGrabbed`
  ;[1 1 1] InputMapping
  (`self.SetActorTickEnabled` true)
  (`self.EnableInput` (`GameplayStatics.GetPlayerController` 0))
  (`EnhancedInputSubsystemInterface.AddMappingContext` (pcsubsystem `EnhancedInputLocalPlayerSubsystem` (`GameplayStatics.GetPlayerController` 0)) "/Game/System/Input/Wand/IMC_Wand_Right.IMC_Wand_Right" 1 (struct))
  (goto _label_2))

(event `self.GrabComponentLeft.OnDropped`
  ;[1 1 1] InputMapping
  (`self.SetActorTickEnabled` true)
  (`self.DisableInput` (`GameplayStatics.GetPlayerController` 0))
  (`EnhancedInputSubsystemInterface.RemoveMappingContext` (pcsubsystem `EnhancedInputLocalPlayerSubsystem` (`GameplayStatics.GetPlayerController` 0)) null (struct))
  (`self.SetActorTickEnabled` false :!label _label_3)
  (`self.SetActorTickEnabled` (`self.BP IDCard`) false)
  (`self.SetActorTickEnabled` (`self.BP_Gate_Right`) false)
  (`self.SetActorTickEnabled` (`self.BP_Gate_Left`) false)
  (`self.SetActorTickEnabled` (`self.BP NPC`) false)
  (bind _bp_how_to_play (`self.BP How To Play`)
    (:`then`
      (`self.SetActorTickEnabled` _bp_how_to_play false))
    (:`else`
      _))
  (`SceneComponent.K2_AttachToComponent` (`self.SM_Wand`) (`self.DefaultSceneRoot`) "None" "SnapToTarget" "SnapToTarget" "KeepWorld" true))

(event `self.GrabComponentRight.OnDropped`
  ;[1 1 1] InputMapping
  (`self.SetActorTickEnabled` true)
  (`self.DisableInput` (`GameplayStatics.GetPlayerController` 0))
  (`EnhancedInputSubsystemInterface.RemoveMappingContext` (pcsubsystem `EnhancedInputLocalPlayerSubsystem` (`GameplayStatics.GetPlayerController` 0)) null (struct))
  (goto _label_3))

(fn `AimObject`
  (params (HitActor :type "Actor Object Reference"))
  (bind _bp_how_to_play (`self.BP How To Play`))
  (bind _bp_idcard (`self.BP IDCard`))
  (bind _bp_npc (`self.BP NPC`))
  (bind _bp_gate_right (`self.BP_Gate_Right`))
  (bind _bp_gate_left (`self.BP_Gate_Left`))
  (bind _asbp_gate_right (cast `/Game/Blueprints/BP_Gate_Right` HitActor)
    (:`then`
      (`/Engine/EditorBlueprintResources/StandardMacros.IsValid` _asbp_gate_right
        (:`Is Valid`
          (set `/Game/Blueprints/BP_Gate_Right.IsAimed` true (`self.BP_Gate_Right`))
          (set `self.AimedObject` "NewEnumerator5"))))
    (:`CastFailed`
      (`|ExecutionSequence`
        (:`then_0`
          (`/Engine/EditorBlueprintResources/StandardMacros.IsValid` _bp_gate_right
            (:`Is Valid`
              (set `/Game/Blueprints/BP_Gate_Right.IsAimed` false _bp_gate_right))))
        (:`then_1`
          (bind _asbp_idcard (cast `/Game/Blueprints/BP_IDCard` HitActor)
            (:`then`
              (`/Engine/EditorBlueprintResources/StandardMacros.IsValid` _asbp_idcard
                (:`Is Valid`
                  (set `/Game/Blueprints/BP_IDCard.IsAimed` true (`self.BP IDCard`))
                  (set `self.AimedObject` "NewEnumerator2"))))
            (:`CastFailed`
              (`|ExecutionSequence`
                (:`then_0`
                  (`/Engine/EditorBlueprintResources/StandardMacros.IsValid` _bp_idcard
                    (:`Is Valid`
                      (set `/Game/Blueprints/BP_IDCard.IsAimed` false _bp_idcard))))
                (:`then_1`
                  (bind _asbp_npc (cast `/Game/NPC/BP_NPC` HitActor)
                    (:`then`
                      (`/Engine/EditorBlueprintResources/StandardMacros.IsValid` _asbp_npc
                        (:`Is Valid`
                          (set `/Game/NPC/BP_NPC.IsAimed` true (`self.BP NPC`))
                          (set `self.AimedObject` "NewEnumerator6"))))
                    (:`CastFailed`
                      (`|ExecutionSequence`
                        (:`then_0`
                          (`/Engine/EditorBlueprintResources/StandardMacros.IsValid` _bp_npc
                            (:`Is Valid`
                              (set `/Game/NPC/BP_NPC.IsAimed` false _bp_npc))))
                        (:`then_1`
                          (bind _asbp_how_to_play (cast `/Game/Blueprints/BP_HowToPlay` HitActor)
                            (:`then`
                              (`/Engine/EditorBlueprintResources/StandardMacros.IsValid` _asbp_how_to_play
                                (:`Is Valid`
                                  (set `/Game/Blueprints/BP_HowToPlay.IsAimed` true (`self.BP How To Play`))
                                  (set `self.AimedObject` "NewEnumerator7"))))
                            (:`CastFailed`
                              (`|ExecutionSequence`
                                (:`then_0`
                                  (`/Engine/EditorBlueprintResources/StandardMacros.IsValid` _bp_how_to_play
                                    (:`Is Valid`
                                      (set `/Game/Blueprints/BP_HowToPlay.IsAimed` false _bp_how_to_play))))
                                (:`then_1`
                                  (bind _asbp_gate_left (cast `/Game/Blueprints/BP_Gate_Left` HitActor)
                                    (:`then`
                                      (`/Engine/EditorBlueprintResources/StandardMacros.IsValid` _asbp_gate_left
                                        (:`Is Valid`
                                          (set `/Game/Blueprints/BP_Gate_Left.IsAimed` true (`self.BP_Gate_Left`))
                                          (set `self.AimedObject` "NewEnumerator3"))))
                                    (:`CastFailed`
                                      (`|ExecutionSequence`
                                        (:`then_0`
                                          (`/Engine/EditorBlueprintResources/StandardMacros.IsValid` _bp_gate_left
                                            (:`Is Valid`
                                              (set `/Game/Blueprints/BP_Gate_Left.IsAimed` false _bp_gate_left))))
                                        (:`then_1`
                                          (set `self.AimedObject` "NewEnumerator4"))))))))))))))))))))))

(fn `UserConstructionScript`)