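; BP_Gate_Right is an aim-activated VR gate that swings open and can approve entry for a guest NPC.
; While aimed at, it shows an animated outline overlay, and IsActivated triggers a timeline-driven opening, guarded by DoOnce.
; Opening stops both gates blocking Visibility; once open, it updates the guest and notifies VRPawn if IsGuestIn.
; After a delay it closes, restores blocking and re-arms.
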(event `self.ReceiveBeginPlay`
  (bind _returnvalue (`KismetMaterialLibrary.CreateDynamicMaterialInstance` (`self.M_Highlight_Inst`)))
  (set `self.DMI_Highlight_Inst` _returnvalue)
  (bind _asvrpawn (cast `/Game/Blueprints/VRPawn` (`GameplayStatics.GetPlayerPawn` 0)))
  (`/Engine/EditorBlueprintResources/StandardMacros.IsValid` _asvrpawn
    (:`Is Valid`
      (set `self.VRPawn` _asvrpawn)
      (bind _returnvalue_2 (`GameplayStatics.GetActorOfClass` "/Game/Blueprints/BP_Gate_Left.BP_Gate_Left_C"))
      (set `self.Gate_Left` _returnvalue_2)
      (bind _outactors (`GameplayStatics.GetAllActorsOfClassWithTag` "/Game/NPC/BP_NPC.BP_NPC_C" "guest"))
      (for _array_element _outactors
        (`/Engine/EditorBlueprintResources/StandardMacros.IsValid` _array_element
          (:`Is Valid`
            (set `self.NPC_Guest` _array_element)))))))

(event `Aimed_Highlight`
  (`MeshComponent.SetOverlayMaterial` (`self.SM_Gate`) (`self.DMI_Highlight_Inst`))
  (bind (_direction _time) (`Timeline|Hightlighting` :!via `PlayFromStart`)
    (:`Update`
      (`MaterialInstanceDynamic.SetScalarParameterValue` (`self.DMI_Highlight_Inst`) "LineThickness" (`KismetMathLibrary.Lerp` 0.5 3.0 _time)))))

(event `self.ReceiveTick`
  (params (DeltaSeconds :type "Float (single-precision)"))
  (if (`self.IsAimed`)
    (`|ExecutionSequence`
      (:`then_0`
        (`/Engine/EditorBlueprintResources/StandardMacros.DoOnce` false :!label _label
          (:`Completed`
            (`self.Aimed_Highlight`))))
      (:`then_1`
        (if (`self.IsActivated`)
          ;[1 1 1] GateActivate
          (`/Engine/EditorBlueprintResources/StandardMacros.DoOnce` false :!label _label_2
            (:`Completed`
              (`PrimitiveComponent.SetCollisionResponseToChannel` (`/Game/Blueprints/BP_Gate_Left.SM_Gate` (`self.Gate_Left`)) "ECC_Visibility" "ECR_Ignore")
              (`PrimitiveComponent.SetCollisionResponseToChannel` (`self.SM_Gate`) "ECC_Visibility" "ECR_Ignore")
              (`GameplayStatics.PlaySound2D` "/Game/SFX/SFX_Twinkle.SFX_Twinkle" 1.0 1.0 0.0 null null)
              (bind (_direction _angle) (`Timeline|GateOpen` :!via `PlayFromStart`)
                (:`Update`
                  (`SceneComponent.K2_SetRelativeRotation` (`self.SM_Gate`) (`KismetMathLibrary.RLerp` (struct) (struct :`Yaw` 180.0) _angle) false false))
                (:`Finished`
                  (`|ExecutionSequence`
                    (:`then_0`
                      (if (`self.IsGuestIn`)
                        (set `/Game/NPC/BP_NPC.bLorR` false (`self.NPC_Guest`))
                        (`/Game/Blueprints/VRPawn.ApproveEntry` (`self.VRPawn`))))
                    (:`then_1`
                      (`KismetSystemLibrary.Delay` 4.0)
                      (set `self.IsActivated` false)
                      (bind (_direction_2 _angle_2) (`Timeline|GateClose` :!via `PlayFromStart`)
                        (:`Update`
                          (`SceneComponent.K2_SetRelativeRotation` (`self.SM_Gate`) (`KismetMathLibrary.RLerp` (struct :`Yaw` 180.0) (struct) _angle_2) false false))
                        (:`Finished`
                          (`PrimitiveComponent.SetCollisionResponseToChannel` (`/Game/Blueprints/BP_Gate_Left.SM_Gate` (`self.Gate_Left`)) "ECC_Visibility" "ECR_Block")
                          (`PrimitiveComponent.SetCollisionResponseToChannel` (`self.SM_Gate`) "ECC_Visibility" "ECR_Block")
                          (goto _label_2 :!via `Reset`))))))))))))
    (else
      (`|ExecutionSequence`
        (:`then_0`
          (goto _label :!via `Reset`))
        (:`then_1`
          (`MeshComponent.SetOverlayMaterial` (`self.SM_Gate`) null))))))

(fn `UserConstructionScript`)