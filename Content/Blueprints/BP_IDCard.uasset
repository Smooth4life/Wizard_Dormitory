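; Physics-driven ID card actor with left and right grab snap points, which despawns the BP_HologramGenerator's hologram when grabbed.
; Tick watches externally set state: when aimed at and not reading, a DoOnce applies a dynamic overlay highlight whose line thickness animates by timeline, cleared otherwise.
; Activating it while aimed teleports the card to its BeginPlay transform, briefly suspending physics.
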(event `self.ReceiveBeginPlay`
  (bind _returnvalue (`KismetMaterialLibrary.CreateDynamicMaterialInstance` (`self.M_Highlight_Inst`)))
  (set `self.DMI_Highlight_Inst` _returnvalue)
  (set `self.DefaultTransform` (`self.GetTransform` self)))

(event `self.GrabComponentSnapRight.OnGrabbed`
  (set `self.IsGrabbed_Right` true)
  (bind _returnvalue (`GameplayStatics.GetActorOfClass` "/Game/Blueprints/HoloGen/BP_HologramGenerator.BP_HologramGenerator_C"))
  (`/Game/Blueprints/HoloGen/BP_HologramGenerator.DespawnHolo` _returnvalue))

(event `self.GrabComponentSnapLeft.OnGrabbed`
  (set `self.IsGrabbed_Left` true)
  (bind _returnvalue (`GameplayStatics.GetActorOfClass` "/Game/Blueprints/HoloGen/BP_HologramGenerator.BP_HologramGenerator_C"))
  (`/Game/Blueprints/HoloGen/BP_HologramGenerator.DespawnHolo` _returnvalue))

(event `self.GrabComponentSnapRight.OnDropped`
  (set `self.IsGrabbed_Right` false))

(event `self.GrabComponentSnapLeft.OnDropped`
  (set `self.IsGrabbed_Left` false))

(event `Aimed_Highlight`
  (`MeshComponent.SetOverlayMaterial` (`self.Card`) (`self.DMI_Highlight_Inst`))
  (bind (_direction _time) (`Timeline|Timeline` :!via `PlayFromStart`)
    (:`Update`
      (`MaterialInstanceDynamic.SetScalarParameterValue` (`self.DMI_Highlight_Inst`) "LineThickness" (`KismetMathLibrary.Lerp` 0.5 3.0 _time)))))

(event `self.ReceiveTick`
  (params (DeltaSeconds :type "Float (single-precision)"))
  (bind _card (`self.Card`))
  (if (and (`self.IsAimed`) (not (`self.IsReading`)))
    (`|ExecutionSequence`
      (:`then_0`
        (`/Engine/EditorBlueprintResources/StandardMacros.DoOnce` false :!label _label
          (:`Completed`
            (`self.Aimed_Highlight`))))
      (:`then_1`
        (if (`self.IsActivated`)
          (`PrimitiveComponent.SetSimulatePhysics` _card false)
          (`SceneComponent.K2_SetWorldTransform` _card (`self.DefaultTransform`) false true)
          (`MeshComponent.SetOverlayMaterial` (`self.Card`) null)
          (`KismetSystemLibrary.Delay` 0.2)
          (`PrimitiveComponent.SetSimulatePhysics` _card true)
          (set `self.IsActivated` false))))
    (else
      (`|ExecutionSequence`
        (:`then_0`
          (goto _label :!via `Reset`))
        (:`then_1`
          (`MeshComponent.SetOverlayMaterial` (`self.Card`) null))))))

(fn `UserConstructionScript`)