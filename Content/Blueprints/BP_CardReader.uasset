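; BP_CardReader is a VR card reader that takes an inserted ID card and shows a hologram of an NPC's affiliation.
; Box overlap, gated by a DoOnce, releases the card from either hand, snaps it to the reader and plays a sound.
; After a short delay, it spawns the hologram through BP_HologramGenerator, choosing the UMG_Hologram display from the first "original"-tagged NPC's affiliation.
; Removing the card clears its reading state and re-arms the reader.
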(event `self.Box.OnComponentBeginOverlap`
  (params (OverlappedComponent :type "PrimitiveComponent Object Reference") (OtherActor :type "Actor Object Reference") (OtherComp :type "PrimitiveComponent Object Reference") (OtherBodyIndex :type Integer) (bFromSweep :type Boolean) (SweepResult :type "HitResult Structure (by ref)"))
  (bind _asbp_idcard (cast `/Game/Blueprints/BP_IDCard` OtherActor))
  (`/Engine/EditorBlueprintResources/StandardMacros.IsValid` _asbp_idcard
    (:`Is Valid`
      (`/Engine/EditorBlueprintResources/StandardMacros.DoOnce` false :!label _label
        (:`Completed`
          (bind _output_get (set `self.IDCard` _asbp_idcard))
          (bind _asvrpawn (cast `/Game/Blueprints/VRPawn` (`GameplayStatics.GetPlayerPawn` 0)))
          (if (`/Game/Blueprints/BP_IDCard.IsGrabbed_Right` _asbp_idcard)
            (bind _breleased (`/Game/Blueprints/GrabComponent.TryRelease` (`/Game/Blueprints/BP_IDCard.GrabComponentSnapRight` _asbp_idcard)))
            (if _breleased
              (set `/Game/Blueprints/VRPawn.HeldComponentRight` null _asvrpawn)
              (set `/Game/Blueprints/BP_IDCard.IsGrabbed_Right` false _asbp_idcard)
              (bind _card (`/Game/Blueprints/BP_IDCard.Card` _asbp_idcard))
              (`PrimitiveComponent.SetSimulatePhysics` _card false :!label _label_2)
              (`SceneComponent.K2_AttachToComponent` _card (`self.CardAttachPos`) "None" "SnapToTarget" "SnapToTarget" "KeepWorld" true)
              (`GameplayStatics.PlaySound2D` "/Game/SFX/SFX_CardReading.SFX_CardReading" 1.0 1.0 0.0 null null)
              (`KismetSystemLibrary.Delay` 0.5)
              (bind _returnvalue (`GameplayStatics.GetActorOfClass` "/Game/Blueprints/HoloGen/BP_HologramGenerator.BP_HologramGenerator_C"))
              (`/Game/Blueprints/HoloGen/BP_HologramGenerator.SpawnHolo` _returnvalue)
              (bind _asumg_hologram (cast `/Game/Blueprints/HoloGen/UMG_Hologram` (`WidgetComponent.GetWidget` (`/Game/Blueprints/HoloGen/BP_HologramGenerator.Widget1` _returnvalue))))
              (`/Engine/EditorBlueprintResources/StandardMacros.IsValid` _asumg_hologram
                (:`Is Valid`
                  (bind _outactors (`GameplayStatics.GetAllActorsOfClassWithTag` "/Game/NPC/BP_NPC.BP_NPC_C" "original"))
                  (switch `int` (`NPC.NPCAffiliationIndex` (`|GetArrayItem` _outactors))
                    (:`0`
                      (`/Game/Blueprints/HoloGen/UMG_Hologram.Luminas` _asumg_hologram))
                    (:`1`
                      (`/Game/Blueprints/HoloGen/UMG_Hologram.Celesta` _asumg_hologram))
                    (:`2`
                      (`/Game/Blueprints/HoloGen/UMG_Hologram.Novas` _asumg_hologram))
                    (:`3`
                      (`/Game/Blueprints/HoloGen/UMG_Hologram.Aurora` _asumg_hologram)))
                  (set `/Game/Blueprints/BP_IDCard.IsReading` true (`self.IDCard`)))))
            (elif (`/Game/Blueprints/BP_IDCard.IsGrabbed_Left` _asbp_idcard)
              (bind _breleased_2 (`/Game/Blueprints/GrabComponent.TryRelease` (`/Game/Blueprints/BP_IDCard.GrabComponentSnapLeft` _asbp_idcard)))
              (if _breleased_2
                (set `/Game/Blueprints/VRPawn.HeldComponentLeft` null _asvrpawn)
                (set `/Game/Blueprints/BP_IDCard.IsGrabbed_Left` false _output_get)
                (goto _label_2))
              (else
                (goto _label_2)))))))))

(event `self.Box.OnComponentEndOverlap`
  (params (OverlappedComponent :type "PrimitiveComponent Object Reference") (OtherActor :type "Actor Object Reference") (OtherComp :type "PrimitiveComponent Object Reference") (OtherBodyIndex :type Integer))
  (bind _asbp_idcard (cast `/Game/Blueprints/BP_IDCard` OtherActor))
  (`/Engine/EditorBlueprintResources/StandardMacros.IsValid` _asbp_idcard
    (:`Is Valid`
      (set `/Game/Blueprints/BP_IDCard.IsReading` false _asbp_idcard)
      (set `self.IDCard` null)
      (`KismetSystemLibrary.Delay` 0.2)
      (goto _label :!via `Reset`))))

(fn `UserConstructionScript`)