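; BP_HologramGenerator is a hologram projector that shows and hides a widget, with a grabbable generator that snaps back to the root when dropped.
; SpawnHolo activates Niagara and scales the widget up with a timeline, then plays a sound.
; DespawnHolo stops the sound and reverses the timeline, hiding widget and particles on finish.
; Paired DoOnce gates block repeat triggers; only the right-grab drop disables physics before reattaching.
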(event `SpawnHolo`
  (bind _niagara (`self.Niagara`))
  (bind _widget1 (`self.Widget1`))
  (`/Engine/EditorBlueprintResources/StandardMacros.DoOnce` false :!label _label
    (:`Completed`
      (`|ExecutionSequence`
        (:`then_0`
          (set `self.Condition` true)
          (`SceneComponent.SetVisibility` _widget1 true true)
          (`ActorComponent.Activate` _niagara true)
          (bind (_direction _newtrack_1) (`Timeline|Timeline` :!via `PlayFromStart` :!label _label_2)
            (:`Update`
              (`SceneComponent.SetRelativeScale3D` _widget1 (* _newtrack_1 (`self.Relative Scale 3D`))))
            (:`Finished`
              (if (`self.Condition`)
                (`AudioComponent.Play` (`self.SFX_Holo`) 0.0)
                (else
                  (`ActorComponent.Deactivate` _niagara)
                  (`NiagaraComponent.ResetSystem` _niagara)
                  (`SceneComponent.SetVisibility` _widget1 false true))))))
        (:`then_1`
          (goto _label_3 :!via `Reset`))))))

(event `DespawnHolo`
  (`/Engine/EditorBlueprintResources/StandardMacros.DoOnce` true :!label _label_3
    (:`Completed`
      (`|ExecutionSequence`
        (:`then_0`
          (set `self.Condition` false)
          (goto _label_2 :!via `ReverseFromEnd`))
        (:`then_1`
          (goto _label :!via `Reset`))
        (:`then_2`
          (`AudioComponent.Stop` (`self.SFX_Holo`)))))))

(event `self.ReceiveBeginPlay`
  (set `self.Relative Scale 3D` (`SceneComponent.RelativeScale3D` (`self.Widget1`))))

(event `self.GrabComponentSnapRight.OnDropped`
  (bind _generator (`self.Generator`))
  (`PrimitiveComponent.SetSimulatePhysics` _generator false)
  (`SceneComponent.K2_AttachToComponent` _generator (`self.DefaultSceneRoot`) "None" "SnapToTarget" "SnapToTarget" "KeepWorld" true :!label _label_4))

(event `self.GrabComponentSnapLeft.OnDropped`
  (goto _label_4))

(fn `UserConstructionScript`)