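; BP_HowToPlay is a tutorial cube that highlights when aimed at and teleports to a tutorial point when activated.
; BeginPlay creates the highlight material, stores the location of an actor tagged Tutorial and calls HowToPlaySpawn on BP_Wand.
; Tick polls IsAimed, using a DoOnce to start a timeline that animates overlay outline thickness.
; Activation while aimed briefly disables physics, moves the cube and clears the highlight.
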(event `self.ReceiveBeginPlay`
  (bind _returnvalue (`KismetMaterialLibrary.CreateDynamicMaterialInstance` (`self.M_Highlight_Inst`)))
  (set `self.DMI_Highlight_Inst` _returnvalue)
  (bind _outactors (`GameplayStatics.GetAllActorsWithTag` "Tutorial"))
  (for _array_element _outactors
    (set `self.SpawnPoint` (`self.K2_GetActorLocation` _array_element)))
  (bind _returnvalue_2 (`GameplayStatics.GetActorOfClass` "/Game/Blueprints/Wand/BP_Wand.BP_Wand_C"))
  (`/Game/Blueprints/Wand/BP_Wand.HowToPlaySpawn` _returnvalue_2))

(event `Aimed_Highlight`
  (`MeshComponent.SetOverlayMaterial` (`self.Cube`) (`self.DMI_Highlight_Inst`))
  (bind (_direction _time) (`Timeline|Timeline` :!via `PlayFromStart`)
    (:`Update`
      (`MaterialInstanceDynamic.SetScalarParameterValue` (`self.DMI_Highlight_Inst`) "LineThickness" (`KismetMathLibrary.Lerp` 0.5 3.0 _time)))))

(event `self.ReceiveTick`
  (params (DeltaSeconds :type "Float (single-precision)"))
  (bind _cube (`self.Cube`))
  (if (`self.IsAimed`)
    (`|ExecutionSequence`
      (:`then_0`
        (`/Engine/EditorBlueprintResources/StandardMacros.DoOnce` false :!label _label
          (:`Completed`
            (`self.Aimed_Highlight`))))
      (:`then_1`
        (if (`self.IsActivated`)
          (`PrimitiveComponent.SetSimulatePhysics` _cube false)
          (`SceneComponent.K2_SetWorldLocationAndRotation` :`self` _cube :`NewLocation` (`self.SpawnPoint`) :`bTeleport` true)
          (`MeshComponent.SetOverlayMaterial` _cube null)
          (`KismetSystemLibrary.Delay` 0.2)
          (`PrimitiveComponent.SetSimulatePhysics` _cube true)
          (set `self.IsActivated` false))))
    (else
      (`|ExecutionSequence`
        (:`then_0`
          (goto _label :!via `Reset`))
        (:`then_1`
          (`MeshComponent.SetOverlayMaterial` (`self.Cube`) null))))))

(fn `UserConstructionScript`)