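; BP_Gate is a gate actor that highlights when aimed at and swings open when activated, then closes itself.
; Tick polls IsAimed, using a DoOnce to start a timeline that animates LineThickness on a dynamic overlay material, cleared when aim leaves.
; While aimed and IsActivated, an open timeline lerps from the current rotation toward a fixed angle.
; After a delay, it clears IsActivated and a close timeline lerps back to zero rotation.
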(event `self.ReceiveBeginPlay`
  (bind _returnvalue (`KismetMaterialLibrary.CreateDynamicMaterialInstance` (`self.M_Highlight_Inst`)))
  (set `self.DMI_Highlight_Inst` _returnvalue))

(event `Aimed_Highlight`
  (`MeshComponent.SetOverlayMaterial` (`self.Cube`) (`self.DMI_Highlight_Inst`))
  (`MeshComponent.SetOverlayMaterial` (`self.Cylinder`) (`self.DMI_Highlight_Inst`))
  (bind (_direction _time) (`Timeline|Hightlighting` :!via `PlayFromStart`)
    (:`Update`
      (`MaterialInstanceDynamic.SetScalarParameterValue` (`self.DMI_Highlight_Inst`) "LineThickness" (`KismetMathLibrary.Lerp` 0.5 3.0 _time)))))

(event `self.ReceiveTick`
  (params (DeltaSeconds :type "Float (single-precision)"))
  (if (`self.IsAimed`)
    (`|ExecutionSequence`
      (:`then_0`
        (`/Engine/EditorBlueprintResources/StandardMacros.DoOnce` false :!label _label
          (:`Completed`
            (`self.Aimed_Highlight`))))
      (:`then_1`
        (if (`self.IsActivated`)
          ;[1 1 1] GateActivate
          (bind (_direction _angle) (`Timeline|GateOpen`)
            (:`Update`
              (`self.K2_SetActorRotation` (`KismetMathLibrary.RLerp` (`self.K2_GetActorRotation`) (struct :`Yaw` -90.0) _angle)))
            (:`Finished`
              (`KismetSystemLibrary.Delay` 2.0)
              (set `self.IsActivated` false)
              (bind (_direction_2 _angle_2) (`Timeline|GateClose`)
                (:`Update`
                  (`self.K2_SetActorRotation` (`KismetMathLibrary.RLerp` (`self.K2_GetActorRotation`) (struct) _angle_2)))))))))
    (else
      (`|ExecutionSequence`
        (:`then_0`
          (goto _label :!via `Reset`))
        (:`then_1`
          (`MeshComponent.SetOverlayMaterial` (`self.Cube`) null)
          (`MeshComponent.SetOverlayMaterial` (`self.Cylinder`) null))))))

(fn `UserConstructionScript`)