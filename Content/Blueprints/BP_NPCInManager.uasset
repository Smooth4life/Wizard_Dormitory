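; BP_NPCInManager is a trigger volume that tracks whether an NPC guest is inside it and updates the gates and entrances to match.
; On BeginPlay it caches both gates, the tagged InDoor and OutDoor entrances, and the VR pawn.
; NPC overlaps set or clear the guest flags on gates and pawn.
; On exit, the NPC's YorN flag selects which entrance's box generates overlap events, disabling the other.
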(event `self.ReceiveBeginPlay`
  (bind _returnvalue (`GameplayStatics.GetActorOfClass` "/Game/Blueprints/BP_Gate_Left.BP_Gate_Left_C"))
  (set `self.Gate_L` _returnvalue)
  (bind _returnvalue_2 (`GameplayStatics.GetActorOfClass` "/Game/Blueprints/BP_Gate_Right.BP_Gate_Right_C"))
  (set `self.Gate_R` _returnvalue_2)
  (bind _outactors (`GameplayStatics.GetAllActorsOfClassWithTag` "/Game/Blueprints/BP_MainEntrance.BP_MainEntrance_C" "InDoor"))
  (for _array_element _outactors
    (set `self.Indoor` _array_element))
  (bind _outactors_2 (`GameplayStatics.GetAllActorsOfClassWithTag` "/Game/Blueprints/BP_MainEntrance.BP_MainEntrance_C" "OutDoor"))
  (for _array_element_2 _outactors_2
    (set `self.Outdoor` _array_element_2))
  (bind _asvrpawn (cast `/Game/Blueprints/VRPawn` (`GameplayStatics.GetPlayerPawn` 0)))
  (`/Engine/EditorBlueprintResources/StandardMacros.IsValid` _asvrpawn
    (:`Is Valid`
      (set `self.VRPawn` _asvrpawn))))

(event `self.Box.OnComponentBeginOverlap`
  (params (OverlappedComponent :type "PrimitiveComponent Object Reference") (OtherActor :type "Actor Object Reference") (OtherComp :type "PrimitiveComponent Object Reference") (OtherBodyIndex :type Integer) (bFromSweep :type Boolean) (SweepResult :type "HitResult Structure (by ref)"))
  (bind _asbp_npc (cast `/Game/NPC/BP_NPC` OtherActor))
  (`/Engine/EditorBlueprintResources/StandardMacros.IsValid` _asbp_npc
    (:`Is Valid`
      (set `/Game/Blueprints/BP_Gate_Left.IsGuestIn` true (`self.Gate_L`))
      (set `/Game/Blueprints/BP_Gate_Right.IsGuestIn` true (`self.Gate_R`))
      (set `/Game/Blueprints/VRPawn.bIsNPCIn` true (`self.VRPawn`)))))

(event `self.Box.OnComponentEndOverlap`
  (params (OverlappedComponent :type "PrimitiveComponent Object Reference") (OtherActor :type "Actor Object Reference") (OtherComp :type "PrimitiveComponent Object Reference") (OtherBodyIndex :type Integer))
  (bind _asbp_npc (cast `/Game/NPC/BP_NPC` OtherActor))
  (`/Engine/EditorBlueprintResources/StandardMacros.IsValid` _asbp_npc
    (:`Is Valid`
      (set `/Game/Blueprints/BP_Gate_Left.IsGuestIn` false (`self.Gate_L`))
      (set `/Game/Blueprints/BP_Gate_Right.IsGuestIn` false (`self.Gate_R`))
      (set `/Game/Blueprints/VRPawn.bIsNPCIn` false (`self.VRPawn`))
      (if (`/Game/NPC/BP_NPC.bYorN` _asbp_npc)
        (set `PrimitiveComponent.bGenerateOverlapEvents` false (`/Game/Blueprints/BP_MainEntrance.Box` (`self.Indoor`)))
        (set `PrimitiveComponent.bGenerateOverlapEvents` true (`/Game/Blueprints/BP_MainEntrance.Box` (`self.Outdoor`)))
        (else
          (set `PrimitiveComponent.bGenerateOverlapEvents` true (`/Game/Blueprints/BP_MainEntrance.Box` (`self.Indoor`)))
          (set `PrimitiveComponent.bGenerateOverlapEvents` false (`/Game/Blueprints/BP_MainEntrance.Box` (`self.Outdoor`))))))))

(fn `UserConstructionScript`)