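; BP_Radio is a radio actor with grabbable dials, apparently for motion-controller hand interaction to adjust volume.
; StartGrab stores the controller, dial and both starting rotations, then reparents the hand mesh onto the dial and enables tick.
; EndGrab snaps the hand back to the controller and disables tick.
; While grabbed, Tick calls UpdateVolume, which is still an empty stub, so the saved rotations go unused.
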(event `self.ReceiveTick`
  (params (DeltaSeconds :type "Float (single-precision)"))
  (if (`self.IsGrabbed`)
    (`self.UpdateVolume`)))

(event `StartGrab`
  (params (Controller :type "MotionControllerComponent Object Reference") (DialComponent :type "StaticMeshComponent Object Reference") (HandMesh :type "SkeletalMeshComponent Object Reference"))
  (if (`self.IsGrabbed`)
    (bind _output_get (set `self.GrabController` Controller))
    (set `self.GrabStartedCtrlRot` (`SceneComponent.K2_GetComponentRotation` _output_get))
    (bind _output_get_2 (set `self.GrabbedDialComponent` DialComponent))
    (set `self.GrabStartedDialRot` (`SceneComponent.RelativeRotation` _output_get_2))
    (set `self.Hand Mesh` HandMesh)
    (set `self.IsGrabbed` true)
    (`SceneComponent.K2_DetachFromComponent` HandMesh "KeepRelative" "KeepRelative" "KeepRelative" true)
    (`SceneComponent.K2_AttachToComponent` HandMesh _output_get_2 "None" "KeepWorld" "KeepWorld" "KeepWorld" true)
    (`self.SetActorTickEnabled` true)))

(event `EndGrab`
  (bind _hand_mesh (`self.Hand Mesh`))
  (if (`self.IsGrabbed`)
    (set `self.IsGrabbed` false)
    (`SceneComponent.K2_DetachFromComponent` _hand_mesh "KeepRelative" "KeepRelative" "KeepRelative" true)
    (`SceneComponent.K2_AttachToComponent` _hand_mesh (`self.GrabController`) "None" "SnapToTarget" "SnapToTarget" "SnapToTarget" true)
    (set `self.GrabController` null)
    (set `self.GrabbedDialComponent` null)
    (`self.SetActorTickEnabled` false)))

(event `UpdateVolume`)

(fn `UserConstructionScript`)