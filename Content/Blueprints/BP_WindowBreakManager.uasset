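; BP_WindowBreakManager is a trigger that plays the LS_BrokenWindow level sequence when a BP_NPC begins overlapping its Box.
; The first valid overlap creates and stores the sequence player through a DoOnce, and every valid overlap then calls Play on it.
; When playback finishes, the player pauses and sets its playback position from PlaybackParams.
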(event `self.Box.OnComponentBeginOverlap`
  (params (OverlappedComponent :type "PrimitiveComponent Object Reference") (OtherActor :type "Actor Object Reference") (OtherComp :type "PrimitiveComponent Object Reference") (OtherBodyIndex :type Integer) (bFromSweep :type Boolean) (SweepResult :type "HitResult Structure (by ref)"))
  (bind _asbp_npc (cast `/Game/NPC/BP_NPC` OtherActor))
  (`/Engine/EditorBlueprintResources/StandardMacros.IsValid` _asbp_npc
    (:`Is Valid`
      (`|ExecutionSequence`
        (:`then_0`
          (`/Engine/EditorBlueprintResources/StandardMacros.DoOnce` false
            (:`Completed`
              (bind (_outactor _returnvalue) (`LevelSequencePlayer.CreateLevelSequencePlayer` "/Game/VFX/BrokenWindow/LS_BrokenWindow.LS_BrokenWindow"))
              (set `self.LevelSequencePlayer` _returnvalue))))
        (:`then_1`
          (`MovieSceneSequencePlayer.Play` (`self.LevelSequencePlayer`)))))))

(event `self.LevelSequencePlayer.OnFinished`
  (bind _levelsequenceplayer (`self.LevelSequencePlayer`))
  (`MovieSceneSequencePlayer.Pause` _levelsequenceplayer)
  (`MovieSceneSequencePlayer.SetPlaybackPosition` _levelsequenceplayer (`self.Playback Params`)))

(fn `UserConstructionScript`)