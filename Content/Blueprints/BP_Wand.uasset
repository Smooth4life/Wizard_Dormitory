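; BP_Wand is a grabbable VR wand that traces a line forward from its muzzle.
; Grabbing and dropping via GrabComponentSnap toggle input and add or remove the Enhanced Input mapping context chosen by holding hand.
; Tick runs a debug-drawn visibility trace with its result unused, and both grab and drop set tick enabled.
; Left and right click events check the holding hand but perform no action yet.
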(event `EnhancedInput|/Game/Input/Wand/Action/IA_Wand_Click_Left`
  (params (ActionValue :type Boolean) (ElapsedSeconds :type "Float (double-precision)") (TriggeredSeconds :type "Float (double-precision)") (InputAction :type "InputAction Object Reference" :default "/Game/Input/Wand/Action/IA_Wand_Click_Left.IA_Wand_Click_Left"))
  (:`Started`
    (if (`|EnumEquality` (`/Game/VRTemplate/Blueprints/GrabComponent.GetHeldByHand` (`self.GrabComponentSnap`)) "Left")
      _)))

(event `EnhancedInput|/Game/Input/Wand/Action/IA_Wand_Click_Right`
  (params (ActionValue :type Boolean) (ElapsedSeconds :type "Float (double-precision)") (TriggeredSeconds :type "Float (double-precision)") (InputAction :type "InputAction Object Reference" :default "/Game/Input/Wand/Action/IA_Wand_Click_Right.IA_Wand_Click_Right"))
  (:`Started`
    (if (`|EnumEquality` (`/Game/VRTemplate/Blueprints/GrabComponent.GetHeldByHand` (`self.GrabComponentSnap`)) "Right")
      _)))

(event `self.ReceiveTick`
  (params (DeltaSeconds :type "Float (single-precision)"))
  (bind _wandmuzzlelocation (`self.WandMuzzleLocation`))
  (bind _returnvalue (`SceneComponent.K2_GetComponentLocation` _wandmuzzlelocation))
  (bind _outhit (`KismetSystemLibrary.LineTraceSingle` :`Start` _returnvalue :`End` (+ _returnvalue (* (`KismetMathLibrary.GetForwardVector` (`SceneComponent.K2_GetComponentRotation` _wandmuzzlelocation)) 10000.0)) :`TraceChannel` "TraceTypeQuery1" :`DrawDebugType` "ForOneFrame")))

(event `self.GrabComponentSnap.OnGrabbed`
  ;[1 1 1] InputMapping
  (`self.SetActorTickEnabled` true)
  (`self.EnableInput` (`GameplayStatics.GetPlayerController` 0))
  (`EnhancedInputSubsystemInterface.AddMappingContext` (pcsubsystem `EnhancedInputLocalPlayerSubsystem` (`GameplayStatics.GetPlayerController` 0)) (select `bool` (`|EnumEquality` (`/Game/VRTemplate/Blueprints/GrabComponent.GetHeldByHand` (`self.GrabComponentSnap`)) "Right") :`false` "/Game/Input/Wand/IMA_Wand_Left.IMA_Wand_Left" :`true` "/Game/Input/Wand/IMA_Wand_Right.IMA_Wand_Right" :!type "InputMappingContext Object Reference") 1 (struct)))

(event `self.GrabComponentSnap.OnDropped`
  ;[1 1 1] InputMapping
  (`self.SetActorTickEnabled` true)
  (`self.DisableInput` (`GameplayStatics.GetPlayerController` 0))
  (`EnhancedInputSubsystemInterface.RemoveMappingContext` (pcsubsystem `EnhancedInputLocalPlayerSubsystem` (`GameplayStatics.GetPlayerController` 0)) (select `bool` (`|EnumEquality` (`/Game/VRTemplate/Blueprints/GrabComponent.GetHeldByHand` (`self.GrabComponentSnap`)) "Right") :`false` "/Game/Input/Wand/IMA_Wand_Left.IMA_Wand_Left" :`true` "/Game/Input/Wand/IMA_Wand_Right.IMA_Wand_Right" :!type "InputMappingContext Object Reference") (struct)))

(fn `UserConstructionScript`)