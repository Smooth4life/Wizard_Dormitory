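; VR telephone prop with a grabbable handset that rings as a tutorial cue on game day 1.
; After a one-second delay it checks BP_GameInstance's day and, on day 1, raises and shakes the phone via a timeline until grabbed.
; Either grab component triggers handset sounds, with delayed PhoneAudio outside the tutorial.
; Dropping snaps the handle back without physics, switches PhoneAudio to line noise and ends the tutorial state.
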(event `self.ReceiveBeginPlay`
  (bind _phone (`self.Phone`))
  (`KismetSystemLibrary.Delay` 1.0)
  (bind _asbp_game_instance (cast `/Game/System/BP_GameInstance` (`GameplayStatics.GetGameInstance`)))
  (if (== (`MyGameInstance.CurrentDay` _asbp_game_instance) 1)
    (set `self.IsTutorial` true)
    (`AudioComponent.Play` (`self.Phone_Ring`) 0.0)
    (bind _output_get (set `self.Relative Location Phone` (`SceneComponent.RelativeLocation` _phone)))
    (`SceneComponent.K2_SetRelativeLocation` _phone (+ _output_get (0.0 0.0 10.0)) false false)
    (bind (_direction _rot) (`Timeline|Timeline` :!label _label)
      (:`Update`
        (`SceneComponent.K2_SetRelativeRotation` _phone (`KismetMathLibrary.MakeRotator` 0.0 _rot) false false)))
    (else
      (`AudioComponent.SetSound` (`self.Phone_Ring`) "/Game/SFX/SFX_PickupTelephone.SFX_PickupTelephone")
      (set `self.IsTutorial` false))))

(event `StopTimeline`
  (goto _label :!via `Stop`))

(event `self.GrabComponentRight.OnGrabbed`
  (bind _phone_ring (`self.Phone_Ring`))
  (if (`self.IsTutorial`) :!label _label_2
    (`|ExecutionSequence`
      (:`then_0`
        (`self.StopTimeline`)
        (`SceneComponent.K2_SetRelativeLocationAndRotation` :`self` (`self.Phone`) :`NewLocation` (`self.Relative Location Phone`))
        (`AudioComponent.Stop` (`self.Phone_Ring`)))
      (:`then_1`
        (`AudioComponent.SetSound` _phone_ring "/Game/SFX/SFX_DropTelephone.SFX_DropTelephone" :!label _label_3)
        (`AudioComponent.Play` _phone_ring 0.0)
        (`KismetSystemLibrary.Delay` 0.8)
        (`AudioComponent.SetSound` _phone_ring "/Game/SFX/SFX_DropTelephone.SFX_DropTelephone")
        (if (not (`self.IsTutorial`))
          (`AudioComponent.Play` (`self.Phone_Audio`) 0.0))))
    (else
      (goto _label_3))))

(event `self.GrabComponentSnapLeft.OnGrabbed`
  (goto _label_2))

(event `self.GrabComponentRight.OnDropped`
  (bind _handle (`self.Handle`))
  (`PrimitiveComponent.SetSimulatePhysics` _handle false :!label _label_4)
  (`SceneComponent.K2_AttachToComponent` _handle (`self.Phone`) "None" "SnapToTarget" "SnapToTarget" "KeepWorld" true)
  (`AudioComponent.Play` (`self.Phone_Ring`) 0.0)
  (`AudioComponent.SetSound` (`self.Phone_Audio`) "/Game/SFX/SFX_TelephoneNoise.SFX_TelephoneNoise")
  (`/Engine/EditorBlueprintResources/StandardMacros.DoOnce` false
    (:`Completed`
      (set `self.IsTutorial` false))))

(event `self.GrabComponentSnapLeft.OnDropped`
  (goto _label_4))

(fn `UserConstructionScript`)